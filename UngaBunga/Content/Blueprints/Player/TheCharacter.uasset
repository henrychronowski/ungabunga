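; Player character for an isometric-camera brawler, with world-axis movement, dash, health, death and pause menus, and HUD.
; Primary and secondary attacks sphere-trace ahead to snap facing toward enemies, then play montages from a shared three-step combo that chains on repeated presses.
; Separate events toggle damage on the spawned, socket-attached weapon, grab or drop enemies, and drive timeline launches that stop when the dash collision overlaps something.
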(event OnComponentBeginOverlap(DashCollision)
  (params (OverlappedComponent :type Primitive%20Component%20Object%20Reference) (OtherActor :type Actor%20Object%20Reference) (OtherComp :type Primitive%20Component%20Object%20Reference) (OtherBodyIndex :type Integer) (bFromSweep :type Boolean) (SweepResult :type Hit%20Result%20Structure%20%28by%20ref%29))
  ;[1 0.838 0.3518] Collision Checks
  (Variables|Default|SetHitBlockingObject true)
  (Variables|/Script/Engine.PrimitiveComponent|SetbGenerateOverlapEvents (Variables|Default|GetDashCollision) false))

(event Custom|TakeDamage
  (params (Amount :type Float%20%28single-precision%29) (Time :type Float%20%28single-precision%29) (Type :type Boolean))
  ;[0.7188 1 0.7065] Health Management
  (Variables|Default|Sethealth (- (Variables|Default|Gethealth) Amount))
  (Effects|SpawnEmitterAttached "/Game/ParticleEffects/Hit.Hit" (Variables|Default|GetCapsuleComponent) "None")
  (if (<= (Variables|Default|Gethealth) 0.0)
    (Variables|Default|Sethealth 0.0)
    (Effects|SpawnEmitteratLocation "/Game/DEFAULT/StarterContent/Particles/P_Explosion.P_Explosion" (Transformation|GetActorLocation))
    (CallFunction|CharacterDeath)))

(event Custom|AddHUDToViewport
  ;[1 1 1] UI
  (CallFunction|HUDAdd "/Game/Widgets/PlayerHud.PlayerHud_C"))

(event Custom|RailPrimaryChain
  (if (Variables|Default|GetChainAttack)
    (CallFunction|DropGrabbedEnemy)
    (Variables|Default|SetChainAttack false)
    (switch int (Variables|Default|GetCombo)
      (:0
        (Variables|Default|SetCombo 1)
        (Variables|Default|SetCurMainMontage "/Game/Animation/Montages/AM_RailMain.AM_RailMain"))
      (:1
        (Variables|Default|SetCombo 2)
        (Variables|Default|SetCurMainMontage "/Game/Animation/Montages/AM_PunchMain.AM_PunchMain"))
      (:2
        (Variables|Default|SetCurMainMontage "/Game/Animation/Montages/AM_PunchMain_NOCHAIN.AM_PunchMain_NOCHAIN")))
    (Animation|Montage|PlayMontage (Variables|Character|GetMesh) (Variables|Default|GetCurMainMontage))))

(event Custom|RailSecondary
  (if (Variables|Default|GetIsSecondarying)
    (Variables|Default|SetChainAttack true)
    (else
      (Variables|Default|SetIsSecondarying true)
      (switch int (Variables|Default|GetCombo)
        (:0
          (Variables|Default|SetCombo 1)
          (Variables|Default|SetCurMainMontage "/Game/Animation/Montages/AM_RailHMain.AM_RailHMain"))
        (:1
          (Variables|Default|SetCombo 2)
          (Variables|Default|SetCurMainMontage "/Game/Animation/Montages/AM_PunchMain.AM_PunchMain"))
        (:2
          (Variables|Default|SetCurMainMontage "/Game/Animation/Montages/AM_PunchMain_NOCHAIN.AM_PunchMain_NOCHAIN")))
      (Animation|Montage|PlayMontage (Variables|Character|GetMesh) (Variables|Default|GetCurMainMontage)))))

(event Custom|GrabEnemy
  (params (EnemyToGrab :type BP%20Base%20Enemy%20Object%20Reference%20%28by%20ref%29))
  (bind _mesh (Variables|Character|GetMesh))
  ;[1 1 1] Grabbing
  (if (and (Utilities|IsValid EnemyToGrab) (not (Utilities|IsValid (Variables|Default|GetCurGrabbedEnemy))))
    (Variables|Default|SetCurGrabbedEnemy EnemyToGrab)
    (Transformation|SetActorLocation (Variables|Default|GetCurGrabbedEnemy) (Transformation|GetSocketLocation _mesh "Railgun_Light") false false)
    (Transformation|AttachComponentToComponent (Variables|Default|GetCurGrabbedEnemy) _mesh "Railgun_Light" "KeepWorld" "KeepWorld" "KeepWorld" false)))

(event Custom|DropGrabbedEnemy
  ;[1 1 1] Grabbing
  (Utilities|IsValid (Variables|Default|GetCurGrabbedEnemy)
    (:Is%20Valid
      (Transformation|DetachFromActor (Variables|Default|GetCurGrabbedEnemy) "KeepWorld" "KeepWorld" "KeepWorld")
      (Default|ResetPositionAfterGrab (Variables|Default|GetCurGrabbedEnemy))
      (Variables|Default|SetCurGrabbedEnemy 0))))

(event Custom|Dash
  (Animation|PlayAnimMontage "/Game/Animation/Montages/TMP_Dash_Montage.TMP_Dash_Montage" 1.0 "None"))

(event Custom|LaunchMeThatWay
  (params (Dir :type Vector) (Scale :type Float%20%28single-precision%29) (Time :type Float%20%28single-precision%29))
  ;[0.7552 0.8027 1] Movement
  ;;[1 1 1] Launch
  (Components|Timeline|SetTimelineLength (Variables|Default|GetLaunchTimeline) Time)
  (Timeline|LaunchTimeline PlayFromStart
    (:Update
      (if (Variables|Default|GetHitBlockingObject)
        (Class|WeaponBase|SetCanHit (Variables|Default|GetWeaponSlot_1) false)
        (Variables|Default|SetHitBlockingObject false)
        (Audio|Components|Audio|Stop (Variables|Default|GetLaunchTimeline))
        (else
          (Character|LaunchCharacter (* Dir Scale) false false))))))

(event Custom|AttackOver
  ;[1 0.7812 0.7812] Attacks
  (Variables|Default|SetIsPrimarying false)
  (Variables|Default|SetIsSecondarying false)
  (Class|WeaponBase|SetCanHit (Variables|Default|GetWeaponSlot_1) false))

(event Custom|CharacterDeath
  (bind _returnvalue (Game|GetPlayerController 0))
  ;[0.7188 1 0.7065] Health Management
  (bind _returnvalue_2 (UserInterface|CreateWidget "/Game/Widgets/DeathMenu.DeathMenu_C"))
  (Variables|/Script/Engine.PlayerController|SetbShowMouseCursor _returnvalue true)
  (Input|SetInputModeUIOnly _returnvalue _returnvalue_2 "DoNotLock")
  (UserInterface|Viewport|AddtoViewport _returnvalue_2 0))

(event Custom|ResetChain
  (Variables|Default|SetIsPrimarying false)
  (Variables|Default|SetIsSecondarying false)
  (Variables|Default|SetChainAttack false)
  (Variables|Default|SetCombo 0)
  (Default|StopAttack (Variables|Default|GetWeaponSlot_1))
  (CallFunction|DropGrabbedEnemy))

(event Custom|RailPrimary
  (if (Variables|Default|GetIsPrimarying)
    (Variables|Default|SetChainAttack true)
    (else
      (Variables|Default|SetIsPrimarying true)
      (switch int (Variables|Default|GetCombo)
        (:0
          (Variables|Default|SetCombo 1)
          (Variables|Default|SetCurMainMontage "/Game/Animation/Montages/AM_RailMain.AM_RailMain"))
        (:1
          (Variables|Default|SetCombo 2)
          (Variables|Default|SetCurMainMontage "/Game/Animation/Montages/AM_PunchMain.AM_PunchMain"))
        (:2
          (Variables|Default|SetCurMainMontage "/Game/Animation/Montages/AM_PunchMain_NOCHAIN.AM_PunchMain_NOCHAIN")))
      (Animation|Montage|PlayMontage (Variables|Character|GetMesh) (Variables|Default|GetCurMainMontage)))))

(event Custom|EnableDamaging
  ;[1 0.7812 0.7812] Attacks
  (Default|SecondaryAttack (Variables|Default|GetWeaponSlot_1) true))

(event Custom|DisableDamaging
  ;[1 0.7812 0.7812] Attacks
  (Default|StopAttack (Variables|Default|GetWeaponSlot_1)))

(event Custom|PlayFootstep
  ;[0.7552 0.8027 1] Movement
  (Audio|PlaySoundatLocation (Variables|Default|GetFootstepCue) "0, 0, 0" "0, 0, 0" 1.0 1.0 0.0 0 0 0))

(event EventBeginPlay
  (Variables|Default|Sethealth (Variables|Default|GetmaxHealth))
  (CallFunction|SpawnWeapon)
  (Input|SetInputModeGameOnly (Game|GetPlayerController 0))
  (Variables|/Script/Engine.PrimitiveComponent|SetbGenerateOverlapEvents (Variables|Default|GetDashCollision) false))

(event EventTick
  (params (DeltaSeconds :type Float%20%28single-precision%29))
  ;[0.7552 0.8027 1] Movement
  (Pawn|Input|AddMovementInput "1.000000, 0, 0" (Input|AxisValues|GetMoveForward) false)
  (Pawn|Input|AddMovementInput "0,1.000000, 0" (Input|AxisValues|GetMoveRight) false))

(event Input|ActionEvents|InputActionPickUp
  (params (Key :type Key%20Structure :default "None")))

(event Input|ActionEvents|InputActionSecondaryAttack
  (params (Key :type Key%20Structure :default "None"))
  (bind _hitcastheightoffset (Variables|Default|GetHitCastHeightOffset))
  (bind _capsulecomponent (Variables|Default|GetCapsuleComponent))
  (bind _returnvalue (Transformation|GetWorldLocation _capsulecomponent))
  (bind _returnvalue_2 (Math|Vector|GetForwardVector _capsulecomponent))
  (bind _returnvalue_3 (+ _hitcastheightoffset _returnvalue))
  ;[1 1 1] Primary
  (:Pressed
    (bind _outhit (Collision|SphereTraceForObjects (+ (* _returnvalue_2 5e+01) _returnvalue_3) (+ _returnvalue_3 (* _returnvalue_2 5e+02)) (Variables|Default|GetSphereWidth) (Variables|Default|GetTargetableEnemies) false 0 "None"))
    (CallFunction|RailSecondary)
    (bind _asbp_base_enemy (Utilities|Casting|CastToBP_BaseEnemy (.hitactor _outhit)))
    (Transformation|SetWorldRotation (Variables|Default|GetCapsuleComponent) (Math|Rotator|MakeRotator 0.0 0.0 (.yaw (Math|Rotator|FindLookatRotation _returnvalue (Transformation|GetActorLocation _asbp_base_enemy)))) false false)))

(event Input|ActionEvents|InputActionMovementAbility
  (params (Key :type Key%20Structure :default "None"))
  ;[0.7552 0.8027 1] Movement
  (:Pressed
    (Variables|/Script/Engine.PrimitiveComponent|SetbGenerateOverlapEvents (Variables|Default|GetDashCollision) true)
    (if (Variables|Default|GetCanDash)
      (CallFunction|Dash)
      (Variables|Default|SetCanDash false)
      (Utilities|FlowControl|Delay 0.3)
      (Variables|Default|SetCanDash true))))

(event Input|ActionEvents|InputActionPauseMenu
  (params (Key :type Key%20Structure :default "None"))
  ;[1 1 1] UI
  (:Pressed
    (Utilities|TriggerPauseMenu)))

(event Input|ActionEvents|InputActionPrimaryAttack
  (params (Key :type Key%20Structure :default "None"))
  (bind _hitcastheightoffset (Variables|Default|GetHitCastHeightOffset))
  (bind _capsulecomponent (Variables|Default|GetCapsuleComponent))
  (bind _returnvalue (Math|Vector|GetForwardVector _capsulecomponent))
  (bind _returnvalue_2 (Transformation|GetWorldLocation _capsulecomponent))
  (bind _returnvalue_3 (+ _hitcastheightoffset _returnvalue_2))
  ;[1 1 1] Primary
  (:Pressed
    (bind _outhit (Collision|SphereTraceForObjects (+ (* _returnvalue 5e+01) _returnvalue_3) (+ _returnvalue_3 (* _returnvalue 5e+02)) (Variables|Default|GetSphereWidth) (Variables|Default|GetTargetableEnemies) false 0 "None"))
    (CallFunction|RailPrimary)
    (bind _asbp_base_enemy (Utilities|Casting|CastToBP_BaseEnemy (.hitactor _outhit)))
    (Transformation|SetWorldRotation (Variables|Default|GetCapsuleComponent) (Math|Rotator|MakeRotator 0.0 0.0 (.yaw (Math|Rotator|FindLookatRotation _returnvalue_2 (Transformation|GetActorLocation _asbp_base_enemy)))) false false)))

(event Input|KeyboardEvents|M
  (params (Key :type Key%20Structure :default "None"))
  ;[1 1 1] UI
  (:Pressed
    (Utilities|TriggerPauseMenu)))

(event Custom|PlayHitEnemy
  (params (Hit%20sound :type Sound%20Cue%20Object%20Reference%20%28by%20ref%29))
  (Audio|PlaySoundatLocation "/Game/SFX/PunchLand.PunchLand" "0, 0, 0" "0, 0, 0" 1.0 1.0 0.0 0 0 0))

(fn ConstructionScript
  (bind _springarm (Variables|Default|GetSpringArm))
  (Utilities|FlowControl|Sequence
    (:then_0
      (Transformation|SetRelativeRotation (Variables|Default|GetSpringArm) (Math|Rotator|MakeRotator 0.0 (* -1 (|(asind((1/(sqrt(3))))))) (Variables|Default|GetZ%20%28Yaw%29)) false false)
      (Class|CameraComponent|SetOrthoWidth (Variables|Default|GetCamera) (Variables|Default|GetIn%20Ortho%20Width)))
    (:then_1
      (Variables|/Script/Engine.SpringArmComponent|SetTargetArmLength _springarm (Variables|Default|GetCameraDistance))
      (Variables|/Script/Engine.SpringArmComponent|SetSocketOffset _springarm (Variables|Default|GetCameraOffset)))))

(fn TEMPScaleRotatorZ
  (params (RotIn :type Rotator) (Scale :type Float%20%28single-precision%29))
  (return (Math|Rotator|MakeRotator (.roll RotIn) (.pitch RotIn) (* (.yaw RotIn) Scale))))

(fn SpawnWeapon
  (bind _returnvalue (Game|SpawnActorfromClass (Variables|Default|GetWeaponToSpawn) (Variables|Default|GetWeaponSpawnTransform) "AlwaysSpawn" 0 0))
  (bind _output_get (Variables|Default|SetWeaponSlot_1 _returnvalue))
  (Transformation|AttachComponentToComponent _output_get (Variables|Character|GetMesh) "Railgun_Light" "KeepRelative" "KeepRelative" "KeepRelative" true))

(fn TMPGetRemainingSwing
  (return 0.25))

(fn HUDAdd
  (params (Class :type User%20Widget%20Class%20Reference))
  (Utilities|IsValid (Variables|Default|GetHudREF)
    (:Is%20Valid
      _)
    (:Is%20Not%20Valid
      (bind _returnvalue (UserInterface|CreateWidget "/Game/Widgets/PlayerHud.PlayerHud_C"))
      (Variables|Default|SetHudREF _returnvalue)))
  (UserInterface|Viewport|AddtoViewport (Variables|Default|GetHudREF) 0))
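; BP_BaseEnemy is a base enemy character that handles health, damage and death.
; Health fills to max on BeginPlay and on possession.
; Damage attaches a hit emitter and opens a caller-supplied invulnerability window via timer; at zero health the enemy spawns an explosion and destroys itself.
; Helper functions set walk speed and return the direction from the capsule to a target location.
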(event `self.ReceiveBeginPlay`
  (set `self.Health` (`self.MaxHealth`) :!label _label))

(event `self.ReceivePossessed`
  (params (NewController :type "Controller Object Reference"))
  (goto _label))

(event `ResetDamageState`
  (set `self.CanTakeDamage` true))

(event `TakeDamage`
  (params (Amount :type "Float (double-precision)") (InvulnTime :type "Float (double-precision)") (Type :type Boolean))
  (if (`self.CanTakeDamage`)
    (set `self.CanTakeDamage` false)
    (`KismetSystemLibrary.K2_SetTimerDelegate` (delegate `ResetDamageState`) InvulnTime)
    (set `self.Health` (- (`self.Health`) Amount))
    (`GameplayStatics.SpawnEmitterAttached` "/Game/ParticleEffects/Hit.Hit" (`self.CapsuleComponent`))
    (if (<= (`self.Health`) 0.0)
      (`KismetSystemLibrary.PrintString` "AI be dead")
      (set `self.Health` 0.0)
      (`GameplayStatics.SpawnEmitterAtLocation` "/Game/DEFAULT/StarterContent/Particles/P_Explosion.P_Explosion" (`self.K2_GetActorLocation`))
      (`self.K2_DestroyActor`))))

(fn `UpdateDirection`
  (params (TargetLocation :type "Vector Structure"))
  (returns (UnitDirection :type "Vector Structure"))
  (return (`KismetMathLibrary.GetDirectionUnitVector` (`SceneComponent.K2_GetComponentLocation` (`self.CapsuleComponent`)) TargetLocation)))

(fn `UpdateWalkSpeed`
  (params (NewWalkSpeed :type "Float (double-precision)"))
  (set `CharacterMovementComponent.MaxWalkSpeed` NewWalkSpeed (`self.CharacterMovement`)))

(fn `UserConstructionScript`)
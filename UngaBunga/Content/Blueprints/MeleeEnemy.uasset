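; MeleeEnemy is a melee enemy that attacks with a montage and damages TheCharacter through a hit box.
; The box starts without collision, switches to query-only on Attack, and switches off again on the montage node's immediate exec output, not on completion.
; An overlap with TheCharacter calls its TakeDamage with HitDamage and also disables the box.
; A separate Stunned event plays a stun montage.
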(event `self.ReceiveBeginPlay`
  (`parent.ReceiveBeginPlay`)
  (`PrimitiveComponent.SetCollisionEnabled` (`self.Box`) "NoCollision"))

(event `Attack`
  (bind _box (`self.Box`))
  (`PrimitiveComponent.SetCollisionEnabled` _box "QueryOnly")
  (`|PlayMontage` (`self.Mesh`) "/Game/Animation/Seeker/AttackMontage.AttackMontage"
    (:`then`
      (`PrimitiveComponent.SetCollisionEnabled` _box "NoCollision" :!label _label))))

(event `self.Box.OnComponentBeginOverlap`
  (params (OverlappedComponent :type "PrimitiveComponent Object Reference") (OtherActor :type "Actor Object Reference") (OtherComp :type "PrimitiveComponent Object Reference") (OtherBodyIndex :type Integer) (bFromSweep :type Boolean) (SweepResult :type "HitResult Structure (by ref)"))
  (bind _asthe_character (cast `/Game/Blueprints/Player/TheCharacter` OtherActor))
  (`/Game/Blueprints/Player/TheCharacter.TakeDamage` _asthe_character (`self.HitDamage`) 0.0 false)
  (goto _label))

(event `Stunned`
  (`|PlayMontage` (`self.Mesh`) "/Game/Blueprints/EnemyAnimations/Stunned.Stunned"))

(fn `UserConstructionScript`
  (`parent.UserConstructionScript`))
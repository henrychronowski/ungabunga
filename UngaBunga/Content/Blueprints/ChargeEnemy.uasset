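; Charging enemy that winds up, rushes at raised speed and damages the player's character on overlap.
; Charge plays a windup montage, then raises walk speed on completion.
; While the ChargeController blackboard's AIState marks a charge, hitting anything but another enemy stops it with a stun montage, and overlapping the player while active deals damage and stops it.
; CheckOverlaps reports whether at least five actors overlap.
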(event `self.ReceiveBeginPlay`
  (`parent.ReceiveBeginPlay`))

(event `self.ReceiveHit`
  (params (MyComp :type "PrimitiveComponent Object Reference") (Other :type "Actor Object Reference") (OtherComp :type "PrimitiveComponent Object Reference") (bSelfMoved :type Boolean) (HitLocation :type "Vector Structure") (HitNormal :type "Vector Structure") (NormalImpulse :type "Vector Structure") (Hit :type "HitResult Structure (by ref)"))
  (cast `/Game/Blueprints/BP_BaseEnemy` Other
    (:`CastFailed`
      (bind _ascharge_controller (cast `/Game/Blueprints/AIBlueprints/ChargeController` (`AIBlueprintHelperLibrary.GetAIController` self)))
      (if (== (`BlackboardComponent.GetValueAsEnum` (`AIBlueprintHelperLibrary.GetBlackboard` _ascharge_controller) (`self.AIState`)) 1)
        (`/Game/Blueprints/AIBlueprints/ChargeController.StopCharge` _ascharge_controller)
        (`|PlayMontage` (`self.Mesh`) "/Game/Animation/Charger/ChargerStunMontage.ChargerStunMontage")))))

(event `self.ReceiveActorBeginOverlap`
  (params (OtherActor :type "Actor Object Reference"))
  (if (`self.IsActive`)
    (bind _ascharge_controller (cast `/Game/Blueprints/AIBlueprints/ChargeController` (`AIBlueprintHelperLibrary.GetAIController` self)))
    (if (== (`BlackboardComponent.GetValueAsEnum` (`AIBlueprintHelperLibrary.GetBlackboard` _ascharge_controller) (`self.AIState`)) 1)
      (bind _asthe_character (cast `/Game/Blueprints/Player/TheCharacter` OtherActor))
      (`/Game/Blueprints/Player/TheCharacter.TakeDamage` _asthe_character (`self.ChargeDamage`) 0.0 false)
      (`/Game/Blueprints/AIBlueprints/ChargeController.StopCharge` _ascharge_controller))))

(event `Charge`
  (`|PlayMontage` (`self.Mesh`) "/Game/Animation/Charger/WindupMontage.WindupMontage"
    (:`OnCompleted`
      (`self.UpdateWalkSpeed` (`self.ChargeSpeed`)))))

(fn `CheckOverlaps`
  (returns (IsOverlapping :type Boolean))
  (if (`KismetArrayLibrary.Array_IsValidIndex` (`self.GetOverlappingActors` "/Script/Engine.Actor") 4)
    (return true)
    (else
      (return false))))

(fn `UserConstructionScript`)
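; Behavior tree task that sets an enemy's TargetDirection blackboard vector to a point offset from the player.
; It passes player zero's location to the EnemyCharacter's UpdateDirection and adds the returned direction, scaled on X and Y only, to that location.
; The task finishes successfully even when the controlled pawn is not an EnemyCharacter, leaving the blackboard untouched.
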(event `self.ReceiveExecuteAI`
  (params (OwnerController :type "AIController Object Reference") (ControlledPawn :type "Pawn Object Reference"))
  (bind _returnvalue (`SceneComponent.K2_GetComponentLocation` (`Actor.RootComponent` (`GameplayStatics.GetPlayerPawn` 0))))
  (bind _asenemy_character (cast `/Game/Blueprints/EnemyCharacter` ControlledPawn)
    (:`then`
      (bind _unitdirection (`/Game/Blueprints/EnemyCharacter.UpdateDirection` _asenemy_character _returnvalue))
      (`BlackboardComponent.SetValueAsVector` (`AIBlueprintHelperLibrary.GetBlackboard` ControlledPawn) (`self.TargetDirection`) (+ _returnvalue (* _unitdirection (1500.0 1500.0 1.0))))
      (`self.FinishExecute` true))
    (:`CastFailed`
      (`self.FinishExecute` true))))
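; AI controller for MeleeEnemy pawns that runs the BTMelee behavior tree.
; On BeginPlay it caches the pawn, stores the player character as its target and writes the initial AIState enum to the blackboard.
; A looping timer fires a Test event that repeatedly forces the state to one fixed enum value.
; Pawn_Attack forwards attack calls to the controlled enemy.
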(event `self.ReceiveBeginPlay`
  (bind _asmelee_enemy (cast `/Game/Blueprints/MeleeEnemy` (`self.K2_GetPawn`)))
  (set `self.EnemyPawn` _asmelee_enemy)
  (`self.RunBehaviorTree` "/Game/Blueprints/AIBlueprints/BTMelee.BTMelee")
  (set `self.CurrentTarget` (`GameplayStatics.GetPlayerCharacter` 0))
  (`BlackboardComponent.SetValueAsEnum` (`AIBlueprintHelperLibrary.GetBlackboard` null) "AIState" (`self.CurrentState`))
  (`KismetSystemLibrary.K2_SetTimerDelegate` (delegate `Test`) 4.0 true))

(event `Test`
  (bind _output_get (set `self.CurrentState` "NewEnumerator1"))
  (`BlackboardComponent.SetValueAsEnum` (`AIBlueprintHelperLibrary.GetBlackboard` null) "AIState" _output_get))

(event `Pawn_Attack`
  (`/Game/Blueprints/MeleeEnemy.Attack` (`self.EnemyPawn`)))

(fn `UserConstructionScript`)
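; Fight director that chooses which melee enemy attacks the player, on a looping timer.
; Each enemy in EnemyList starts with a random grade, shown on a debug widget component attached to it.
; Each tick of the timer scales grades by a forward-vector dot product, favoring enemies facing opposite to the player's facing.
; The top-graded enemy's MeleeController triggers its attack, then that enemy's grade is rerolled.
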(event `self.ReceiveBeginPlay`
  (for _array_element (`self.EnemyList`)
    (bind _asmelee_enemy (cast `/Game/Blueprints/MeleeEnemy` _array_element))
    (`self.AddDebugWidgets` _asmelee_enemy))
  (`KismetSystemLibrary.K2_SetTimerDelegate` (delegate `TriggerAttack`) 4.0 true))

(event `TriggerAttack`
  (`self.RecalculateScores`)
  (bind (_lockhighestvalue1 _lockhighestgradedai1) (`self.FindHighestGrade`))
  (bind _asmelee_controller (cast `/Game/Blueprints/AIBlueprints/MeleeController` (`AIBlueprintHelperLibrary.GetAIController` _lockhighestgradedai1)))
  (`/Game/Blueprints/AIBlueprints/MeleeController.AIAttack` _asmelee_controller)
  (`BlueprintMapLibrary.Map_Add` (`self.EnemyGrading`) _lockhighestgradedai1 (`KismetMathLibrary.RandomFloatInRange` 1.0 5.0))
  (`self.UpdateDebugWidgets` _lockhighestgradedai1))

(fn `AddDebugWidgets`
  (params (EnemyInstance :type "/Game/Blueprints/MeleeEnemy Object Reference (by ref)"))
  (locals (Loc_Widget :type "/Game/Blueprints/AIBlueprints/DebugMeleeAI Object Reference"))
  (bind _enemyinstance (`local.EnemyInstance`))
  (bind _enemyinstance_2 (`local.EnemyInstance`))
  (`BlueprintMapLibrary.Map_Add` (`self.EnemyGrading`) EnemyInstance (`KismetMathLibrary.RandomFloatInRange` 1.0 5.0))
  (bind _returnvalue (`|CreateWidget` "/Game/Blueprints/AIBlueprints/DebugMeleeAI.DebugMeleeAI_C" null _enemyinstance (`BlueprintMapLibrary.Map_Find` (`self.EnemyGrading`) _enemyinstance)))
  (bind _output_get (set `local.Loc_Widget` _returnvalue))
  (`BlueprintMapLibrary.Map_Add` (`self.EnemyWidgets`) _enemyinstance_2 _output_get)
  (bind _returnvalue_2 (`AddComponent|NODE_AddWidgetComponent-0` :`self` _enemyinstance_2))
  (`WidgetComponent.SetWidget` _returnvalue_2 (`local.Loc_Widget`)))

(fn `FindHighestGrade`
  (returns (LockHighestValue1 :type "Float (double-precision)") (LockHighestGradedAI1 :type "/Game/Blueprints/MeleeEnemy Object Reference"))
  (locals (LockHighestValue :type "Float (double-precision)") (LockHighestGradedAI :type "/Game/Blueprints/MeleeEnemy Object Reference"))
  (bind _keys (`BlueprintMapLibrary.Map_Keys` (`self.EnemyGrading`)))
  (for _array_element _keys
    (bind _asmelee_enemy (cast `/Game/Blueprints/MeleeEnemy` _array_element))
    (bind _value (`BlueprintMapLibrary.Map_Find` (`self.EnemyGrading`) _asmelee_enemy))
    (if (> _value (`local.LockHighestValue`))
      (set `local.LockHighestValue` _value)
      (set `local.LockHighestGradedAI` _asmelee_enemy)))
  (return (`local.LockHighestValue`) (`local.LockHighestGradedAI`)))

(fn `RecalculateScores`
  (`self.ScoreByPosition`))

(fn `ScoreByPosition`
  (bind _enemygrading (`self.EnemyGrading`))
  (for _array_element (`self.EnemyList`)
    (bind _asmelee_enemy (cast `/Game/Blueprints/MeleeEnemy` _array_element))
    (`BlueprintMapLibrary.Map_Add` _enemygrading _asmelee_enemy (* (`BlueprintMapLibrary.Map_Find` _enemygrading _asmelee_enemy) (+ (`KismetMathLibrary.NormalizeToRange` (* (`KismetMathLibrary.Dot_VectorVector` (`self.GetActorForwardVector` _asmelee_enemy) (`self.GetActorForwardVector` (`GameplayStatics.GetPlayerCharacter` 0))) -1.0) -1.0 1.0) 0.5)))
    (`self.UpdateDebugWidgets` _asmelee_enemy)))

(fn `UpdateDebugWidgets`
  (params (EnemyInstance :type "/Game/Blueprints/MeleeEnemy Object Reference"))
  (set `/Game/Blueprints/AIBlueprints/DebugMeleeAI.FightingGrade` (`BlueprintMapLibrary.Map_Find` (`self.EnemyGrading`) EnemyInstance) (`BlueprintMapLibrary.Map_Find` (`self.EnemyWidgets`) EnemyInstance)))

(fn `UserConstructionScript`)
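; AI controller for the ChargeEnemy pawn that starts a charge when it sees the player.
; ActivateAI runs the BTChargeEnemy behavior tree, targets the player character and mirrors the current state into the AIState Blackboard key.
; Once active, sighting a Player-tagged actor advances that state and disables sight, latching the trigger.
; StopCharge writes ChargeState back to the Blackboard, and Tick's perceived-actor loop only casts, with no effect.
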(event `self.ActivateAI`
  (`self.RunBehaviorTree` "/Game/Blueprints/AIBlueprints/BTChargeEnemy.BTChargeEnemy")
  (set `self.CurrentTarget` (`GameplayStatics.GetPlayerCharacter` 0))
  (`BlackboardComponent.SetValueAsEnum` (`AIBlueprintHelperLibrary.GetBlackboard` null) "AIState" (`self.CurrentState`))
  (set `self.isActive` true))

(event `self.ReceiveBeginPlay`
  (bind _ascharge_enemy (cast `/Game/Blueprints/ChargeEnemy` (`self.K2_GetPawn`)))
  (set `self.EnemyPawn` _ascharge_enemy))

(event `self.ReceiveTick`
  (params (DeltaSeconds :type "Float (single-precision)"))
  (if true
    (if (== (`self.CurrentState`) 0)
      (for _array_element (`AIPerceptionComponent.GetPerceivedActors` (`self.AIPerception`) "/Script/AIModule.AISense_Sight")
        (cast `/Game/Blueprints/Player/TheCharacter` _array_element)))))

(event `self.AIPerception.OnTargetPerceptionUpdated`
  (params (Actor :type "Actor Object Reference") (Stimulus :type "AIStimulus Structure"))
  (if (`self.isActive`)
    (if (and (`.bSuccessfullySensed` (break `AIStimulus` Stimulus)) (`self.ActorHasTag` Actor "Player"))
      (bind _output_get (set `self.CurrentState` "NewEnumerator1"))
      (`BlackboardComponent.SetValueAsEnum` (`AIBlueprintHelperLibrary.GetBlackboard` null) "AIState" _output_get)
      (`KismetSystemLibrary.PrintString` "ChargeStarted")
      (`AIPerceptionComponent.SetSenseEnabled` (`self.GetAIPerceptionComponent`) "/Script/AIModule.AISense_Sight" false))))

(fn `StopCharge`
  (locals (ChargeState :type "/Game/Blueprints/AIBlueprints/ChargeState Enum" :default "NewEnumerator2"))
  (`BlackboardComponent.SetValueAsEnum` (`self.Blackboard`) (`self.AIState`) (`local.ChargeState`)))

(fn `UserConstructionScript`)
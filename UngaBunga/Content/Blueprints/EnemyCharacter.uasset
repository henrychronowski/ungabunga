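; Enemy character Blueprint that pairs with a ChargeController AI controller for a charge behavior.
; On a Hit event it casts its AI controller to ChargeController and stops the charge.
; Helper functions set max walk speed, return a unit direction from the capsule to a target location, and report whether at least five actors overlap the enemy.
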(event `self.ReceiveHit`
  (params (MyComp :type "PrimitiveComponent Object Reference") (Other :type "Actor Object Reference") (OtherComp :type "PrimitiveComponent Object Reference") (bSelfMoved :type Boolean) (HitLocation :type "Vector Structure") (HitNormal :type "Vector Structure") (NormalImpulse :type "Vector Structure") (Hit :type "HitResult Structure (by ref)"))
  (bind _ascharge_controller (cast `/Game/Blueprints/AIBlueprints/ChargeController` (`AIBlueprintHelperLibrary.GetAIController` self)))
  (`/Game/Blueprints/AIBlueprints/ChargeController.StopCharge` _ascharge_controller))

(fn `CheckOverlaps`
  (returns (IsOverlapping :type Boolean))
  (if (`KismetArrayLibrary.Array_IsValidIndex` (`self.GetOverlappingActors` "/Script/Engine.Actor") 4)
    (return true)
    (else
      (return false))))

(fn `UpdateDirection`
  (params (TargetLocation :type "Vector Structure"))
  (returns (UnitDirection :type "Vector Structure"))
  (return (`KismetMathLibrary.GetDirectionUnitVector` (`SceneComponent.K2_GetComponentLocation` (`self.CapsuleComponent`)) TargetLocation)))

(fn `UpdateWalkSpeed`
  (params (NewWalkSpeed :type "Float (double-precision)"))
  (set `CharacterMovementComponent.MaxWalkSpeed` NewWalkSpeed (`self.CharacterMovement`)))

(fn `UserConstructionScript`)
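; DoorManager opens and closes a group of doors around fights, based on the FightManager's enemy list.
; Each Tick with no enemies left, it slides all Doors against the Speed vector until one nears its open position.
; With enemies present, a triggered door makes open doors slide back to 400 units above that position, then activates every enemy's AI.
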(event `self.ReceiveBeginPlay`)

(event `self.ReceiveTick`
  (params (DeltaSeconds :type "Float (single-precision)"))
  (if (== (`KismetArrayLibrary.Array_Length` (`/Game/Blueprints/AIBlueprints/FightDirector.EnemyList` (`self.FightManager`))) 0)
    (if (not (`self.DoorsOpen`))
      (for _array_element (`self.Doors`)
        (bind _returnvalue (`SceneComponent.K2_GetComponentLocation` (`/Game/Blueprints/Door/Door.DefaultSceneRoot` _array_element)))
        (`self.K2_SetActorLocation` _array_element (+ (* (* (`self.Speed`) -1) DeltaSeconds) _returnvalue) false false)
        (bind _openpos (`/Game/Blueprints/Door/Door.Get Open Pos` _array_element))
        (if (== _returnvalue _openpos :`ErrorTolerance` 10.0)
          (set `self.DoorsOpen` true))))
    (else
      (for _array_element_2 (`self.Doors`)
        (if (`/Game/Blueprints/Door/Door.isTriggered` _array_element_2)
          (if (`self.DoorsOpen`)
            (for _array_element_3 (`self.Doors`)
              (bind _returnvalue_2 (`SceneComponent.K2_GetComponentLocation` (`/Game/Blueprints/Door/Door.DefaultSceneRoot` _array_element_3)))
              (`self.K2_SetActorLocation` _array_element_3 (+ _returnvalue_2 (* (`self.Speed`) DeltaSeconds)) false false)
              (bind _openpos_2 (`/Game/Blueprints/Door/Door.Get Open Pos` _array_element_3))
              (if (== _returnvalue_2 (+ _openpos_2 (0.0 0.0 400.0)) :`ErrorTolerance` 10.0)
                (set `self.DoorsOpen` false)
                (for _array_element_4 (`/Game/Blueprints/AIBlueprints/FightDirector.EnemyList` (`self.FightManager`))
                  (`/Game/Blueprints/BP_BaseEnemy.ActivateAI` _array_element_4))))))))))

(fn `UserConstructionScript`)
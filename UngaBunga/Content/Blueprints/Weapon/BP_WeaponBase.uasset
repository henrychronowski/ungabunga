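; Base weapon actor that damages BP_BaseEnemy targets through swept traces, with empty primary and secondary attack events.
; While CanHit is set, each tick line-traces from Tip, Mid and Base to their previous-frame positions, trying the next point only when nothing collides.
; Initial-overlap hits on enemies apply BaseDamage, using the player's remaining swing time as invulnerability time.
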(event `self.ReceiveBeginPlay`
  (bind _asthe_character (cast `/Game/Blueprints/Player/TheCharacter` (`GameplayStatics.GetPlayerPawn` 0)))
  (set `self.PlayerREF` _asthe_character))

(event `self.ReceiveTick`
  (params (DeltaSeconds :type "Float (single-precision)"))
  (if (`self.canHit`)
    (`self.CheckCasts`))
  (`self.UpdatePrev`))

(event `PrimaryAttack`)

(event `SecondaryAttack`)

(fn `CheckCasts`
  (bind _asthe_character (cast `/Game/Blueprints/Player/TheCharacter` (`GameplayStatics.GetPlayerPawn` 0)))
  (bind _remaining (`/Game/Blueprints/Player/TheCharacter.TMPGetRemainingSwing` _asthe_character))
  (set `self.InvulnTime` _remaining)
  (`self.SingleCast` (`SceneComponent.K2_GetComponentLocation` (`self.Tip`)) (`self.TipPrev`) "ForDuration" (struct :`R` 1.0 :`B` 0.778244 :`A` 1.0) 0.5
    (:`NoCollide`
      (`self.SingleCast` (`SceneComponent.K2_GetComponentLocation` (`self.Mid`)) (`self.MidPrev`) "ForDuration" (struct :`R` 0.021329 :`B` 1.0 :`A` 1.0) 0.5
        (:`NoCollide`
          (`self.SingleCast` (`SceneComponent.K2_GetComponentLocation` (`self.Base`)) (`self.BasePrev`) "ForDuration" (struct :`R` 1.0 :`G` 0.769892 :`A` 1.0) 0.5))))))

(fn `UpdatePrev`
  (set `self.TipPrev` (`SceneComponent.K2_GetComponentLocation` (`self.Tip`)))
  (set `self.MidPrev` (`SceneComponent.K2_GetComponentLocation` (`self.Mid`)))
  (set `self.BasePrev` (`SceneComponent.K2_GetComponentLocation` (`self.Base`))))

(fn `UserConstructionScript`)
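; BaseWeapon is a weapon Blueprint with early-stage swept hit detection, toggled through SetCanHit.
; Each Tick while CanHit is set, CheckTraces line-traces on Visibility from the Tip component's previous position to its current one, covering movement between frames.
; UpdatePrevious then stores Tip, Mid and Base positions, though only Tip is traced.
; A hit only prints a debug string; no damage is applied.
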(event `self.ReceiveBeginPlay`)

(event `self.ReceiveTick`
  (params (DeltaSeconds :type "Float (single-precision)"))
  (if (`self.CanHit`)
    (`self.CheckTraces`))
  (`self.UpdatePrevious`))

(fn `CheckTraces`
  (`|ExecutionSequence`
    (:`then_0`
      (bind (_outhit _returnvalue) (`KismetSystemLibrary.LineTraceSingle` (`self.TipPrev`) (`SceneComponent.K2_GetComponentLocation` (`self.Tip`)) "TraceTypeQuery1"))
      (if _returnvalue
        (`KismetSystemLibrary.PrintString` "Hello")))))

(fn `setCanHit`
  (params (Param :type Boolean))
  (set `self.CanHit` Param))

(fn `UpdatePrevious`
  (set `self.TipPrev` (`SceneComponent.K2_GetComponentLocation` (`self.Tip`)))
  (set `self.MidPrev` (`SceneComponent.K2_GetComponentLocation` (`self.Mid`)))
  (set `self.BasePrev` (`SceneComponent.K2_GetComponentLocation` (`self.Base`))))

(fn `UserConstructionScript`)
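; BP_BaseThrowable is a base actor for objects that can be picked up and thrown to damage enemies.
; Throw enables mesh physics and Hitbox overlaps, then applies a mass-independent force with an upward bias.
; Hitbox overlaps damage BP_BaseEnemy actors with a brief invulnerability time, and PickedUp turns physics and overlaps off.
; CanHit is set on throw and cleared on Hitbox hit, but the damage path never checks it.
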(event `TEST_throw`
  (`self.Throw` (0.0 0.0 1.0) 1000.0))

(event `self.Hitbox.OnComponentBeginOverlap`
  (params (OverlappedComponent :type "PrimitiveComponent Object Reference") (OtherActor :type "Actor Object Reference") (OtherComp :type "PrimitiveComponent Object Reference") (OtherBodyIndex :type Integer) (bFromSweep :type Boolean) (SweepResult :type "HitResult Structure (by ref)"))
  (bind _asbp_base_enemy (cast `/Game/Blueprints/BP_BaseEnemy` OtherActor))
  (`/Game/Blueprints/BP_BaseEnemy.TakeDamage` _asbp_base_enemy 20.0 0.5 false))

(event `self.Hitbox.OnComponentHit`
  (params (HitComponent :type "PrimitiveComponent Object Reference") (OtherActor :type "Actor Object Reference") (OtherComp :type "PrimitiveComponent Object Reference") (NormalImpulse :type "Vector Structure") (Hit :type "HitResult Structure (by ref)"))
  (set `self.canHit` false))

(event `PickedUp`
  (bind _staticmesh (`self.StaticMesh`))
  (`PrimitiveComponent.SetSimulatePhysics` _staticmesh false)
  (set `PrimitiveComponent.bGenerateOverlapEvents` false _staticmesh)
  (set `PrimitiveComponent.bGenerateOverlapEvents` false (`self.Hitbox`)))

(fn `Throw`
  (params (Direction :type "Vector Structure" :default (0.0 0.0 1.0)) (Speed :type "Float (double-precision)" :default 50.0))
  (bind _hitbox (`self.Hitbox`))
  (`PrimitiveComponent.SetSimulatePhysics` (`self.StaticMesh`) true)
  (`PrimitiveComponent.AddForce` (`self.StaticMesh`) (* (+ Direction (0.0 0.0 0.6)) Speed) "None" true)
  (set `self.canHit` true)
  (set `PrimitiveComponent.bGenerateOverlapEvents` true _hitbox)
  (set `PrimitiveComponent.bGenerateOverlapEvents` true _hitbox))

(fn `UserConstructionScript`)
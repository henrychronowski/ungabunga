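; Player character with an isometric camera and camera-relative movement.
; The construction script angles the camera at 45° yaw and the true isometric pitch of arcsin(1/√3), then pulls it back by CameraDistance plus CameraOffset.
; Each tick, MoveForward and MoveRight axis inputs drive movement along the camera's yaw-only forward and right vectors.
; A temporary T key binding toggles between orthographic and perspective projection.
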(event EventBeginPlay)

(event Collision|EventActorBeginOverlap
  (params (OtherActor :type Actor%20Object%20Reference)))

(event EventTick
  (params (DeltaSeconds :type Float%20%28single-precision%29))
  (bind _camera (Variables|Default|GetCamera))
  (bind _returnvalue (Transformation|GetWorldRotation _camera))
  (bind _returnvalue_2 (Math|Rotator|MakeRotator 0.0 0.0 (.yaw _returnvalue)))
  (Pawn|Input|AddMovementInput (Math|Vector|GetForwardVector _returnvalue_2) (Input|AxisValues|GetMoveForward) false)
  (Pawn|Input|AddMovementInput (Math|Vector|GetRightVector _returnvalue_2) (Input|AxisValues|GetMoveRight) false))

(event Input|KeyboardEvents|T
  (params (Key :type Key%20Structure :default "None"))
  (:Pressed
    (Utilities|TEMPProjectionSwitch)))

(fn ConstructionScript
  (Utilities|FlowControl|Sequence
    (:then_0
      (Transformation|SetRelativeRotation (Variables|Default|GetCamera) (Math|Rotator|MakeRotator 0.0 (* -1 (|(asind((1/(sqrt(3))))))) 45.0) false false))
    (:then_1
      (Transformation|SetRelativeLocation (Variables|Default|GetCamera) (+ (* (Math|Vector|GetForwardVector (Variables|Default|GetCamera)) (* -1 (Variables|Default|GetCameraDistance))) (Variables|Default|GetCameraOffset)) false false))))
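; Fire light Blueprint that flickers Orange and Yellow lights through timelines scaling the intensities cached at BeginPlay.
; Yellow's curve also gets a random multiplier each update, and each finished timeline restarts its own flicker after a random delay.
; Each start event stops the other timeline, so BeginPlay's back-to-back calls halt Orange's flicker and leave only Yellow's cycle running.
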(event `self.ReceiveBeginPlay`
  (set `self.BaseIntensityOrange` (`LightComponentBase.Intensity` (`self.Orange`)))
  (set `self.BaseIntensityYellow` (`LightComponentBase.Intensity` (`self.Yellow`)))
  (`self.StartFlickerOrange`)
  (`self.StartFlickerYellow`))

(event `StartFlickerOrange`
  (`|ExecutionSequence`
    (:`then_0`
      (bind (_direction _intensity) (`Timeline|Timeline_0` :!via `Stop` :!label _label)
        (:`Update`
          (`LightComponent.SetIntensity` (`self.Yellow`) (* (* _intensity (`KismetMathLibrary.RandomFloatInRange` 0.5 1.5)) (`self.BaseIntensityYellow`))))
        (:`Finished`
          (`KismetSystemLibrary.Delay` (`KismetMathLibrary.RandomFloatInRange` 2.0 10.0))
          (`self.StartFlickerYellow`))))
    (:`then_1`
      (bind (_direction_2 _intensity_2) (`Timeline|Flicker` :!via `PlayFromStart` :!label _label_2)
        (:`Update`
          (`LightComponent.SetIntensity` (`self.Orange`) (* _intensity_2 (`self.BaseIntensityOrange`))))
        (:`Finished`
          (`KismetSystemLibrary.Delay` (`KismetMathLibrary.RandomFloatInRange` 2.0 10.0))
          (`self.StartFlickerOrange`))))))

(event `StartFlickerYellow`
  (`|ExecutionSequence`
    (:`then_0`
      (goto _label_2 :!via `Stop`))
    (:`then_1`
      (goto _label :!via `PlayFromStart`))))

(fn `UserConstructionScript`)